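; GlobalTimer is a world clock actor that drives a day/night cycle from game time and a configurable seconds-per-day length.
; Each Tick it pitches the sun, updates the sky sphere, recaptures the sky light and derives the current day, hour and minute.
; It compares the 6:00–18:00 daytime window with the stored IsDayTime flag to fire EnterDayTime or EnterNightTime on transitions, which currently only print messages.
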(event Custom|EnterNightTime
  (Development|PrintString "天黑了"))

(event Custom|EnterDayTime
  (Development|PrintString "天亮了"))

(event EventBeginPlay)

(event Collision|EventActorBeginOverlap
  (params (OtherActor :type Actor%20Object%20Reference)))

(event EventTick
  (params (DeltaSeconds :type Float%20%28single-precision%29))
  (bind _returnvalue (Utilities|Time|GetGameTimeinSeconds))
  (bind _secondperday (Variables|Default|GetSecondPerDay))
  (bind _returnvalue_2 (/ _secondperday 24.0))
  (bind (_remainder _returnvalue_3) (Math|Float|Division(WholeandRemainder) _returnvalue _secondperday))
  (bind (_remainder_2 _returnvalue_4) (Math|Float|Division(WholeandRemainder) _remainder _returnvalue_2))
  (Transformation|SetActorRotation (Variables|Default|GetSunLight) (Math|Rotator|MakeRotator 0.0 (+ (* -360 (/ _remainder _secondperday)) 9e+01) 0.0))
  (Default|UpdateSunDirection (Variables|Default|GetSkySphere))
  (Class|SkyLightComponent|RecaptureSky (Variables|/Script/Engine.SkyLight|GetLightComponent (Variables|Default|GetSkyLight)))
  (Variables|Default|SetCurrentDay _returnvalue_3)
  (bind _output_get (Variables|Default|SetCurrentHour _returnvalue_4))
  (Variables|Default|SetCurrentMinute (.ReturnValue (Math|Float|Division(WholeandRemainder) _remainder_2 (/ _returnvalue_2 6e+01))))
  (Utilities|FlowControl|Sequence
    (:then_0
      (if (and (< _output_get 18) (>= _output_get 6))
        (if (not (Variables|Default|GetIsDayTime))
          (CallFunction|EnterDayTime))
        (elif (Variables|Default|GetIsDayTime)
          (CallFunction|EnterNightTime))))
    (:then_1
      (Variables|Default|SetIsDayTime (and (< _output_get 18) (>= _output_get 6))))))

(fn ConstructionScript)