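; Weight-limited inventory that stores item slots in a map keyed by name and tracks total Load against Capacity.
; TryAddItem checks weight from the item class defaults via TestCapacity, then adds a slot or increments an existing stack by one, returning Chinese feedback text.
; RemoveItem takes one unit off, basing the new count on the passed-in slot.
; Both call added, removed or count-changed notifications as slots change.
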(fn TestCapacity
  (params (NewItem :type Struct%20Item%20Slot%20Structure))
  (bind (_type _name _icon _count) (Utilities|Struct|BreakStruct_ItemSlot NewItem))
  (bind _load (Variables|Default|GetLoad))
  (bind _weight (Utilities|GetClassDefaults _type))
  (bind _returnvalue (* _weight _count))
  (bind _returnvalue_2 (+ _returnvalue _load))
  (return (>= (Variables|Default|GetCapacity) _returnvalue_2) _returnvalue_2))

(fn TryAddItem
  (params (NewItem :type Struct%20Item%20Slot%20Structure))
  (LocalVariables|SetLocalNewItemName (.Name (Utilities|Struct|BreakStruct_ItemSlot NewItem)))
  (bind _output_get (LocalVariables|SetLocalAddedNewItem NewItem))
  (bind (_success _newload) (CallFunction|TestCapacity _output_get))
  (if _success
    (Variables|Default|SetLoad _newload)
    (if (Utilities|Map|Contains (Variables|Default|GetContent) (LocalVariables|GetLocalNewItemName))
      (LocalVariables|SetLocalNewItemCount (+ (.Count (Utilities|Struct|BreakStruct_ItemSlot (.Value (Utilities|Map|Find (Variables|Default|GetContent) (LocalVariables|GetLocalNewItemName))))) 1))
      (Utilities|Map|Remove (Variables|Default|GetContent) (LocalVariables|GetLocalNewItemName))
      (Utilities|Map|Add (Variables|Default|GetContent) (LocalVariables|GetLocalNewItemName) (Utilities|Struct|MakeStruct_ItemSlot (.Type (Utilities|Struct|BreakStruct_ItemSlot (LocalVariables|GetLocalAddedNewItem))) (.Name (Utilities|Struct|BreakStruct_ItemSlot (LocalVariables|GetLocalAddedNewItem))) (.Icon (Utilities|Struct|BreakStruct_ItemSlot (LocalVariables|GetLocalAddedNewItem))) (LocalVariables|GetLocalNewItemCount)))
      (Default|CallChangedCount (Utilities|Struct|MakeStruct_ItemSlot (.Type (Utilities|Struct|BreakStruct_ItemSlot (LocalVariables|GetLocalAddedNewItem))) (.Name (Utilities|Struct|BreakStruct_ItemSlot (LocalVariables|GetLocalAddedNewItem))) (.Icon (Utilities|Struct|BreakStruct_ItemSlot (LocalVariables|GetLocalAddedNewItem))) (LocalVariables|GetLocalNewItemCount)))
      (return true (Utilities|String|Append "被捡到：" (LocalVariables|GetLocalNewItemName) "  count:" (Utilities|String|ToString(Integer) (LocalVariables|GetLocalNewItemCount))))
      (else
        (Utilities|Map|Add (Variables|Default|GetContent) (LocalVariables|GetLocalNewItemName) (LocalVariables|GetLocalAddedNewItem))
        (Default|CallAddedItem (LocalVariables|GetLocalAddedNewItem))
        (return true (Utilities|String|Append "被捡到：" (LocalVariables|GetLocalNewItemName)))))
    (else
      (return false (Utilities|String|Append "背包满了" "")))))

(fn RemoveItem
  (params (Target :type Struct%20Item%20Slot%20Structure))
  (bind (_type _name _icon _count) (Utilities|Struct|BreakStruct_ItemSlot Target))
  (Development|PrintString 0 "remove item")
  (LocalVariables|SetTargetName _name)
  (if (.ReturnValue (Utilities|Map|Find (Variables|Default|GetContent) (LocalVariables|GetTargetName)))
    (LocalVariables|SetFoundSlot (.Value (Utilities|Map|Find (Variables|Default|GetContent) (LocalVariables|GetTargetName))))
    (Development|PrintString 0 (Utilities|String|Append "current count" (Utilities|String|ToString(Integer) _count)))
    (LocalVariables|SetCurrentCount _count)
    (Utilities|Map|Remove (Variables|Default|GetContent) (LocalVariables|GetTargetName))
    (Variables|Default|SetLoad (Math|Integer|Max(Integer) (- (Variables|Default|GetLoad) (.Weight (Utilities|GetClassDefaults _type)))))
    (if (> (LocalVariables|GetCurrentCount) 1)
      (Development|PrintString 0 (Utilities|String|Append "new name" _name "   new count:  " (Utilities|String|ToString(Integer) (- (LocalVariables|GetCurrentCount) 1)) "   old count:    " (Utilities|String|ToString(Integer) (LocalVariables|GetCurrentCount))))
      (Utilities|Map|Add (Variables|Default|GetContent) (LocalVariables|GetTargetName) (Utilities|Struct|MakeStruct_ItemSlot _type _name _icon (- (LocalVariables|GetCurrentCount) 1)))
      (Default|CallChangedCount (Utilities|Struct|MakeStruct_ItemSlot _type _name _icon (- (LocalVariables|GetCurrentCount) 1)))
      (else
        (Default|CallRemovedItem (LocalVariables|GetFoundSlot))))))