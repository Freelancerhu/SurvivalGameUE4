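; Storage cabinet prop that holds stacked item slots for the survival game.
; A box overlap with the survival character shows or hides the cabinet UI through the game instance and sets the game mode's near-cabinet flag.
; AddItem and RemoveItem keep a name-keyed Content map, rebuilding slots to change stack counts and dropping empty ones.
; Each change fires a dispatcher for added, removed or updated-count items.
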(event OnComponentBeginOverlap(Box)
  (params (OverlappedComponent :type Primitive%20Component%20Object%20Reference) (OtherActor :type Actor%20Object%20Reference) (OtherComp :type Primitive%20Component%20Object%20Reference) (OtherBodyIndex :type Integer) (bFromSweep :type Boolean) (SweepResult :type Hit%20Result%20Structure%20%28by%20ref%29))
  (Utilities|Casting|CastToSurvivalCharacter OtherActor)
  (Default|ShowCabinetUI (.AsSurvival%20Game%20Instance (Utilities|Casting|CastToSurvivalGameInstance (Game|GetGameInstance))))
  (Variables|/Game/Blueprints/SurvivalGameMode.SurvivalGameMode_C|SetPlayerNearCabinet (.AsSurvival%20Game%20Mode (Utilities|Casting|CastToSurvivalGameMode (Game|GetGameMode))) true))

(event OnComponentEndOverlap(Box)
  (params (OverlappedComponent :type Primitive%20Component%20Object%20Reference) (OtherActor :type Actor%20Object%20Reference) (OtherComp :type Primitive%20Component%20Object%20Reference) (OtherBodyIndex :type Integer))
  (Utilities|Casting|CastToSurvivalCharacter OtherActor)
  (Default|HideCabinetUI (.AsSurvival%20Game%20Instance (Utilities|Casting|CastToSurvivalGameInstance (Game|GetGameInstance))))
  (Variables|/Game/Blueprints/SurvivalGameMode.SurvivalGameMode_C|SetPlayerNearCabinet (.AsSurvival%20Game%20Mode (Utilities|Casting|CastToSurvivalGameMode (Game|GetGameMode))) false))

(event EventBeginPlay)

(event Collision|EventActorBeginOverlap
  (params (OtherActor :type Actor%20Object%20Reference)))

(event EventTick
  (params (DeltaSeconds :type Float%20%28single-precision%29)))

(fn ConstructionScript)

(fn AddItem
  (params (NewItem :type Struct%20Item%20Slot%20Structure))
  (bind _output_get (LocalVariables|SetNewAddedItem NewItem))
  (LocalVariables|SetNewAddedName (.Name (Utilities|Struct|BreakStruct_ItemSlot _output_get)))
  (if (Utilities|Map|Contains (Variables|Default|GetContent) (LocalVariables|GetNewAddedName))
    (LocalVariables|SetNewCount (+ (.Count (Utilities|Struct|BreakStruct_ItemSlot (.Value (Utilities|Map|Find (Variables|Default|GetContent) (LocalVariables|GetNewAddedName))))) 1))
    (Utilities|Map|Remove (Variables|Default|GetContent) (LocalVariables|GetNewAddedName))
    (Utilities|Map|Add (Variables|Default|GetContent) (LocalVariables|GetNewAddedName) (Utilities|Struct|MakeStruct_ItemSlot (.type (LocalVariables|GetNewAddedItem)) (.name (LocalVariables|GetNewAddedItem)) (.icon (LocalVariables|GetNewAddedItem)) (LocalVariables|GetNewCount)))
    (Default|CallUpdatedItemCount (Utilities|Struct|MakeStruct_ItemSlot (.type (LocalVariables|GetNewAddedItem)) (.name (LocalVariables|GetNewAddedItem)) (.icon (LocalVariables|GetNewAddedItem)) (LocalVariables|GetNewCount)))
    (return)
    (else
      (Utilities|Map|Add (Variables|Default|GetContent) (LocalVariables|GetNewAddedName) (LocalVariables|GetNewAddedItem))
      (Default|CallAddeditem (LocalVariables|GetNewAddedItem))
      (return))))

(fn RemoveItem
  (params (RemovedItem :type Struct%20Item%20Slot%20Structure))
  (bind _output_get (LocalVariables|SetTheRemovedItem RemovedItem))
  (LocalVariables|SetRemovedItemName (.Name (Utilities|Struct|BreakStruct_ItemSlot _output_get)))
  (if (Utilities|Map|Contains (Variables|Default|GetContent) (LocalVariables|GetRemovedItemName))
    (LocalVariables|SetOldItemCount (.Count (Utilities|Struct|BreakStruct_ItemSlot (.Value (Utilities|Map|Find (Variables|Default|GetContent) (LocalVariables|GetRemovedItemName))))))
    (if (== (- (.Count (Utilities|Struct|BreakStruct_ItemSlot (.Value (Utilities|Map|Find (Variables|Default|GetContent) (LocalVariables|GetRemovedItemName))))) 1) 0)
      (Utilities|Map|Remove (Variables|Default|GetContent) (LocalVariables|GetRemovedItemName))
      (Default|CallRemovedItem (LocalVariables|GetTheRemovedItem))
      (return)
      (else
        (Utilities|Map|Remove (Variables|Default|GetContent) (LocalVariables|GetRemovedItemName))
        (Utilities|Map|Add (Variables|Default|GetContent) (LocalVariables|GetRemovedItemName) (Utilities|Struct|MakeStruct_ItemSlot (.Type (Utilities|Struct|BreakStruct_ItemSlot (LocalVariables|GetTheRemovedItem))) (.Name (Utilities|Struct|BreakStruct_ItemSlot (LocalVariables|GetTheRemovedItem))) (.Icon (Utilities|Struct|BreakStruct_ItemSlot (LocalVariables|GetTheRemovedItem))) (- (LocalVariables|GetOldItemCount) 1)))
        (Default|CallUpdatedItemCount (Utilities|Struct|MakeStruct_ItemSlot (.Type (Utilities|Struct|BreakStruct_ItemSlot (LocalVariables|GetTheRemovedItem))) (.Name (Utilities|Struct|BreakStruct_ItemSlot (LocalVariables|GetTheRemovedItem))) (.Icon (Utilities|Struct|BreakStruct_ItemSlot (LocalVariables|GetTheRemovedItem))) (- (LocalVariables|GetOldItemCount) 1)))
        (return)))
    (else
      (return))))