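; Survival game instance that manages the player's UI panels: runtime UI, messages, pickables, inventory and cabinet.
; ShowPanel lazily creates each widget into a by-ref variable, reuses it afterwards and adds it to the viewport.
; Interactive panels increment ActiveUICount and enable Game-and-UI input with a cursor; HidePanel decrements it and restores game-only input at zero.
; PushMessage forwards text to the message panel.
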(event Custom|CreateRuntimeUI
  (CallFunction|ShowPanel "/Game/UI/UI_RuntimeUI.UI_RuntimeUI_C" (Variables|Default|GetRuntimeUI) false)
  (CallFunction|ShowPanel "/Game/UI/UI_MessagePanel.UI_MessagePanel_C" (Variables|Default|GetMessagePanel) false))

(event Custom|ShowInventoryPanel
  (CallFunction|ShowPanel "/Game/UI/UI_Inventory.UI_Inventory_C" (Variables|Default|GetInventoryPanel) true))

(event Custom|HideInventoryPanel
  (CallFunction|HidePanel (Variables|Default|GetInventoryPanel)))

(event Custom|CreatePickablePanel
  (CallFunction|ShowPanel "/Game/UI/UI_PickablePanel.UI_PickablePanel_C" (Variables|Default|GetPickablePanel) true))

(event Custom|HidePickablePanel
  (CallFunction|HidePanel (Variables|Default|GetPickablePanel)))

(event Custom|PushMessage
  (params (TextContent :type String))
  (Default|PushMessage (Variables|Default|GetMessagePanel) TextContent))

(event Custom|HideCabinetUI
  (CallFunction|HidePanel (Variables|Default|GetCabinetUI)))

(event Custom|ShowCabinetUI
  (CallFunction|ShowPanel "/Game/UI/UI_Cabinet.UI_Cabinet_C" (Variables|Default|GetCabinetUI) true))

(fn SetMouseCursoron
  (bind _returnvalue (Game|GetPlayerController 0))
  (Input|SetInputModeGameandUI _returnvalue (Variables|Default|GetPickablePanel) "DoNotLock" true)
  (Variables|/Script/Engine.PlayerController|SetbShowMouseCursor _returnvalue true))

(fn ShowPanel
  (params (PanelTypeClass :type User%20Widget%20Class%20Reference) (PanelVarible :type User%20Widget%20Object%20Reference%20%28by%20ref%29) (bChangeUIMode :type Boolean))
  (bind _returnvalue (Game|GetPlayerController 0))
  (Utilities|IsValid PanelVarible
    (:Is%20Valid
      (if (not (UserInterface|Viewport|IsinViewport PanelVarible))
        (UserInterface|Viewport|AddtoViewport PanelVarible 0 :!label _label)
        (if bChangeUIMode
          (Math|Integer|IncrementInt (Variables|Default|GetActiveUICount)
            (:%20%20
              (Input|SetInputModeGameandUI _returnvalue PanelVarible "DoNotLock" true)
              (Variables|/Script/Engine.PlayerController|SetbShowMouseCursor _returnvalue true))))))
    (:Is%20Not%20Valid
      (bind _returnvalue_2 (UserInterface|CreateWidget PanelTypeClass (Game|GetPlayerController 0)))
      (|SetBy-RefVar PanelVarible _returnvalue_2)
      (goto _label))))

(fn HidePanel
  (params (TargetPanel :type User%20Widget%20Object%20Reference%20%28by%20ref%29))
  (bind _returnvalue (Game|GetPlayerController 0))
  (Utilities|IsValid TargetPanel
    (:Is%20Valid
      (Widget|RemovefromParent TargetPanel)
      (bind _result (Math|Integer|DecrementInt (Variables|Default|GetActiveUICount))
        (:%20%20
          (if (== _result 0)
            (Input|SetInputModeGameOnly _returnvalue)
            (Variables|/Script/Engine.PlayerController|SetbShowMouseCursor _returnvalue false)))))))